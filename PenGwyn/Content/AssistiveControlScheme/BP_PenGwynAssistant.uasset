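; PenGwyn assistant actor that applies assistive-control options and records player combat telemetry.
; GI_Options sets roll assistance level and enables item assistance, which auto-uses a potion below 50 health on Tick.
; Update events fill a current stats struct, which UpdateAssistance tags with the active spawn point's room ID and archives before calling an empty AnalyseData.
; Fifteen seconds after BeginPlay, it archives once and saves all records to SavedData.json.
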(event `InitalSetAssistance`
  (bind _asbp_third_person_character (cast `/Game/ThirdPerson/Blueprints/BP_ThirdPersonCharacter` (`GameplayStatics.GetPlayerCharacter` 0) :!pure true))
  (`KismetSystemLibrary.PrintString` "Assistance Updated")
  (bind _asgi_options (cast `/Game/Save/GI_Options` (`GameplayStatics.GetGameInstance`)))
  (`|ExecutionSequence`
    (:`then_0`
      (bind (_assistance_levels_itemusage _assistance_levels_rollinvulframe) (break `/Game/AssistiveControlScheme/S_Asistance_Levels` (`/Game/Save/GI_Options.Assistance_Levels` _asgi_options)))
      (switch `/Game/AssistiveControlScheme/E_AssitanceLevel` _assistance_levels_itemusage
        (:`NewEnumerator0`
          (set `self.ItemAssistance` false))
        (:`NewEnumerator1`
          (set `self.ItemAssistance` true :!label _label))
        (:`NewEnumerator2`
          (goto _label))
        (:`NewEnumerator3`
          (goto _label)))
      (`KismetSystemLibrary.PrintString` (`KismetStringLibrary.Conv_BoolToString` (`self.ItemAssistance`))))
    (:`then_1`
      (switch `/Game/AssistiveControlScheme/E_AssitanceLevel` _assistance_levels_rollinvulframe
        (:`NewEnumerator0`
          (set `/Game/ThirdPerson/Blueprints/BP_ThirdPersonCharacter.RollAssistanceLevel` 0 _asbp_third_person_character))
        (:`NewEnumerator1`
          (set `/Game/ThirdPerson/Blueprints/BP_ThirdPersonCharacter.RollAssistanceLevel` 1 _asbp_third_person_character))
        (:`NewEnumerator2`
          (set `/Game/ThirdPerson/Blueprints/BP_ThirdPersonCharacter.RollAssistanceLevel` 2 _asbp_third_person_character))
        (:`NewEnumerator3`
          (set `/Game/ThirdPerson/Blueprints/BP_ThirdPersonCharacter.RollAssistanceLevel` 3 _asbp_third_person_character))))))

(event `TestDataIsSaved`
  ;[0.6302 0 0] Debug tests
  (for _ (range 6)
    (`self.UpdateAssistance`)))

(event `/Game/AssistiveControlScheme/BPI_DataLogging.UpdatePotionUsed`
  ;[0 0.01449 1] Interfaces for updating Current Struct
  (`self.UPDPotions`))

(event `/Game/AssistiveControlScheme/BPI_DataLogging.UpdateLeavesUsed`
  ;[0 0.01449 1] Interfaces for updating Current Struct
  (`self.UPDLeaves`))

(event `/Game/AssistiveControlScheme/BPI_DataLogging.UpdateBalmsUsed`
  ;[0 0.01449 1] Interfaces for updating Current Struct
  (`self.UPDBalms`))

(event `/Game/AssistiveControlScheme/BPI_DataLogging.UpdateNumOfDeaths`
  ;[0 0.01449 1] Interfaces for updating Current Struct
  (`self.UPDNumofDeaths`))

(event `/Game/AssistiveControlScheme/BPI_DataLogging.UpdateTimeTaken`
  (params (Time :type "Float (double-precision)"))
  ;[0 0.01449 1] Interfaces for updating Current Struct
  (`self.UPDTimeTaken` Time))

(event `/Game/AssistiveControlScheme/BPI_DataLogging.UpdateNumOfAttacksBlocked`
  ;[0 0.01449 1] Interfaces for updating Current Struct
  (`self.UPDNumberofAttacksBlocked`))

(event `self.ReceiveBeginPlay`
  (`self.InitalSetAssistance`)
  (`self.CreateJsonFile`)
  (`KismetSystemLibrary.Delay` 15.0)
  (`self.UpdateAssistance`)
  (`self.SetJsonValues`)
  (`self.SaveJsonFile`))

(event `/Game/AssistiveControlScheme/BPI_DataLogging.UpdateAverageTimeBlocking`
  (params (`Average Time` :type "Float (double-precision)"))
  ;[0 0.01449 1] Interfaces for updating Current Struct
  (`self.CalculateAverageBlockTime`))

(event `/Game/AssistiveControlScheme/BPI_DataLogging.UpdateAverageHealthofEnemeisAtEndOfCombat`
  (params (`Average Health` :type "Float (double-precision)"))
  ;[0 0.01449 1] Interfaces for updating Current Struct
  (`self.UPDAverageHealthOfEnemeis` `Average Health`))

(event `/Game/AssistiveControlScheme/BPI_DataLogging.UpdateNumOfEnemiesInCombatAtDeath`
  (params (Num :type "Float (double-precision)"))
  ;[0 0.01449 1] Interfaces for updating Current Struct
  (`self.UPDNumberofEnemeisAlliveAtDeath` Num))

(event `/Game/AssistiveControlScheme/BPI_DataLogging.UpdateNumOf EnemyAttacks`
  ;[0 0.01449 1] Interfaces for updating Current Struct
  (`self.UPDNumberofEnemyattacks`))

(event `Check Player Health`
  (bind _health (message `/Game/DamageSystem/BPI_Damagable.GetCurrentHealth` (`GameplayStatics.GetPlayerCharacter` 0)))
  (set `self.NeedToHeal` (< _health 50.0)))

(event `/Game/AssistiveControlScheme/BPI_DataLogging.UpdateNumOfSuccessfullEnemyAttacks`
  ;[0 0.01449 1] Interfaces for updating Current Struct
  (`self.UPDNumberofEnemyattacksSuccess`))

(event `/Game/AssistiveControlScheme/BPI_DataLogging.UpdateNumOfTimesItemAssistanceUsed`
  ;[0 0.01449 1] Interfaces for updating Current Struct
  (`self.UPDNumberofTimesItemAssistanceUsed`))

(event `PlayerUsePotion`
  (bind _asbp_third_person_character (cast `/Game/ThirdPerson/Blueprints/BP_ThirdPersonCharacter` (`GameplayStatics.GetPlayerCharacter` 0)))
  (`/Game/ThirdPerson/Blueprints/BP_ThirdPersonCharacter.SetInuseItemPotion` _asbp_third_person_character)
  (`KismetSystemLibrary.Delay` 2.0)
  (`/Game/ThirdPerson/Blueprints/BP_ThirdPersonCharacter.UseItem` _asbp_third_person_character)
  (`KismetSystemLibrary.Delay` 4.0)
  (set `self.HealingFlagged` false)
  ;[0 1 0.04705] Data Log
  (`self.UpdateNumOfTimesItemAssistanceUsed`))

(event `/Game/AssistiveControlScheme/BPI_DataLogging.UpdateNumOfTimesTakenDamage`
  ;[0 0.01449 1] Interfaces for updating Current Struct
  (`self.UPDNumberofTimesDamageTaken`))

(event `/Game/AssistiveControlScheme/BPI_DataLogging.UpdateTimeLockOnUsed`
  (params (Time :type "Float (double-precision)"))
  ;[0 0.01449 1] Interfaces for updating Current Struct
  (`self.UPDTimeLockOnUsed` Time))

(event `self.ReceiveTick`
  (params (DeltaSeconds :type "Float (single-precision)"))
  (`self.AssistanceTick`))

(event `/Game/AssistiveControlScheme/BPI_DataLogging.UpdateLockedOnUsed`
  (params (IsUsed :type Boolean))
  ;[0 0.01449 1] Interfaces for updating Current Struct
  (`self.UPDIsLockOnUsed` IsUsed))

(event `AssistanceTick`
  (if (`self.ItemAssistance`)
    (`self.Check Player Health`)
    (if (and (`self.NeedToHeal`) (not (`self.HealingFlagged`)))
      (set `self.HealingFlagged` true)
      (`self.PlayerUsePotion`))))

(event `/Game/AssistiveControlScheme/BPI_DataLogging.UpdateNumOfSuccessfullRolls`
  ;[0 0.01449 1] Interfaces for updating Current Struct
  (`self.UPDNumberofRollSuccess`))

(event `/Game/AssistiveControlScheme/BPI_DataLogging.UpdateNumOfRollAttempts`
  ;[0 0.01449 1] Interfaces for updating Current Struct
  (`self.UPDNumberofRoll`))

(event `UpdateAssistance`
  (`KismetSystemLibrary.PrintString` "Assitance Updated By fog wall")
  (`self.UpdateAverageTimeBlocking` 0.0)
  (`self.UpdateRoomID`)
  (`self.UpdateStoredInfo`)
  (`self.AnalyseData`))

(event `/Game/AssistiveControlScheme/BPI_DataLogging.UpdateNumOfSuccessfullAttacks`
  ;[0 0.01449 1] Interfaces for updating Current Struct
  (`self.UPDNumberofAttackSuccess`))

(event `/Game/AssistiveControlScheme/BPI_DataLogging.UpdateNumOfAttackAttempts`
  ;[0 0.01449 1] Interfaces for updating Current Struct
  (`self.UPDNumberofAttacks`))

(event `/Game/AssistiveControlScheme/BPI_DataLogging.UpdateAverageHealth`
  (params (AverageHealth :type "Float (double-precision)"))
  ;[0 0.01449 1] Interfaces for updating Current Struct
  (`self.CalculateAveragePlayerHealth`))

(event `/Game/AssistiveControlScheme/BPI_DataLogging.AddPlayerHealthValue`
  (params (Value :type "Float (double-precision)"))
  ;[0 0.01449 1] Interfaces for updating Current Struct
  (`self.AddPlayerHealthValues` Value))

(event `/Game/AssistiveControlScheme/BPI_DataLogging.AddBlockTime`
  (params (Timer :type "Float (double-precision)"))
  ;[0 0.01449 1] Interfaces for updating Current Struct
  (`self.AddBlockTimeValues` Timer)
  (`KismetSystemLibrary.PrintString` (`KismetStringLibrary.Conv_DoubleToString` Timer)))

(event `/Game/AssistiveControlScheme/BPI_DataLogging.AddLivingEnemyHealth`
  (params (Value :type "Float (double-precision)"))
  ;[0 0.01449 1] Interfaces for updating Current Struct
)

(fn `AnalyseData`)

(fn `CalculateAverageBlockTime`
  (locals (AverageTimeIndex :type Integer) (AddativeTime :type "Float (double-precision)") (AverageTime :type "Float (double-precision)"))
  (bind _addativetime (`local.AddativeTime`))
  (for _array_element (`self.BlockTimes`)
    (set `local.AddativeTime` (+ (`local.AddativeTime`) _array_element))
    (bind _result (`/Engine/EditorBlueprintResources/StandardMacros.IncrementInt` (`local.AverageTimeIndex`))
      (:`  `
        (set `local.AverageTimeIndex` _result))))
  (bind _output_get (set `local.AverageTime` (/ _addativetime (`local.AverageTimeIndex`))))
  (`self.UPDAverageBlockTime` _output_get
    (:`Update`
      (`self.UPDTotalBlockTime` _addativetime
        (:`Update`
          (set `local.AddativeTime` 0.0))))))

(fn `CalculateAveragePlayerHealth`
  (locals (AverageHealthIndex :type Integer) (AddativeHealth :type "Float (double-precision)") (AverageHealth :type "Float (double-precision)"))
  (for _array_element (`self.HealthValues`)
    (set `local.AddativeHealth` (+ (`local.AddativeHealth`) _array_element))
    (bind _result (`/Engine/EditorBlueprintResources/StandardMacros.IncrementInt` (`local.AverageHealthIndex`))
      (:`  `
        (set `local.AverageHealthIndex` _result))))
  (bind _output_get (set `local.AverageHealth` (/ (`local.AddativeHealth`) (`local.AverageHealthIndex`))))
  (`self.UPDAverageHealth` _output_get
    (:`output`
      (set `local.AddativeHealth` 0.0))))

(fn `CreateJsonFile`
  (bind (_bsuccess _jsonobject) (`JSONUtility.CreateNewJsonObj`))
  (set `self.Main Json` _jsonobject))

(fn `SaveJsonFile`
  (bind (_bsuccess _jsonstring) (`JSONUtility.JsonToString` (`self.Main Json`) true))
  (bind _bsuccess_2 (`GeneralUtility.SaveTextFile` _jsonstring (make `JsonHttpFileData` (`KismetSystemLibrary.GetProjectDirectory`) "SavedData.json")))
  (if _bsuccess_2
    (`KismetSystemLibrary.PrintString` "Save made")
    (else
      (`KismetSystemLibrary.PrintString` "Save Failed"))))

(fn `SetJsonValues`
  (`JSONUtility.SetNewObjectField` (`self.Main Json`) "Stored Data")
  (for _array_element (`self.TrackedDataStorage`)
    (bind (_bsuccess _jsonobject) (`JSONUtility.CreateNewJsonObj`))
    (bind _output_get (set `self.Json Object` _jsonobject))
    (bind _updatejson (`self.SetJsonArrayValue` _array_element _output_get))
    (bind _output_get_2 (set `self.Json Object` _updatejson))
    (`KismetArrayLibrary.Array_Add` (`self.ArrayData`) _output_get_2))
  (`JSONUtility.SetArrayField` (`self.Main Json`) "Saves" false (`self.ArrayData`)))

(fn `UpdateRoomID`
  (bind _outactors (`GameplayStatics.GetAllActorsOfClass` "/Game/Experience/Blueprints/Enviroment/BP_PlayerSpawnPoint.BP_PlayerSpawnPoint_C"))
  (for _array_element _outactors
    (if (`/Game/Experience/Blueprints/Enviroment/BP_PlayerSpawnPoint.IsActive` _array_element)
      (`self.SetRoomID` (`/Game/Experience/Blueprints/Enviroment/BP_PlayerSpawnPoint.Point ID` _array_element))
      (break))))

(fn `UpdateStoredInfo`
  (bind _trackeddatacurrent_saveid (break `/Game/AssistiveControlScheme/S_Tracked_Data` (`self.TrackedDataCurrent`)))
  (`KismetArrayLibrary.Array_Add` (`self.TrackedDataStorage`) (`self.TrackedDataCurrent`))
  (bind _result (`/Engine/EditorBlueprintResources/StandardMacros.IncrementInt` _trackeddatacurrent_saveid)
    (:`  `
      (set `self.TrackedDataCurrent` (make `/Game/AssistiveControlScheme/S_Tracked_Data` _result)))))

(fn `UserConstructionScript`)