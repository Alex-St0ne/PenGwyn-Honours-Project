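; Base enemy Blueprint that gives AI enemies health, stamina, damage handling and a health bar widget.
; BPCStatusComponent owns the stats, with getters, Heal and TakeDamage forwarding to it so the Healthbar widget can receive the enemy as its damageable actor.
; The construction script binds the component's blocked, damage response and death events.
; Hits and blocks only print debug text, while death ragdolls the mesh and destroys the actor after a delay.
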(event `self.ReceiveBeginPlay`
  (bind _returnvalue (`|CreateWidget` "/Game/DamageSystem/UI/Healthbar.Healthbar_C" null self))
  (`WidgetComponent.SetWidget` (`self.HP_Bar`) _returnvalue))

(event `Death`
  (bind _mesh (`self.Mesh`))
  (`KismetSystemLibrary.PrintString` "Dead")
  (`PrimitiveComponent.SetSimulatePhysics` _mesh true)
  (`PrimitiveComponent.SetCollisionEnabled` _mesh "QueryAndPhysics")
  (`KismetSystemLibrary.Delay` 4.0)
  (`self.K2_DestroyActor`))

(event `DamageReaction`
  (params (`Damage Response` :type "/Game/DamageSystem/E_Damage_Response Enum" :default "NewEnumerator0"))
  (`KismetSystemLibrary.PrintString` "Damaged"))

(event `DamageBlocked`
  (`KismetSystemLibrary.PrintString` "Blocked"))

(fn `GetCurrentHealth`
  (returns (Health :type "Float (double-precision)"))
  (return (`/Game/DamageSystem/BPC_StatusComponent.CurrentHealth` (`self.BPC_StatusComponent`))))

(fn `GetCurrentStamina`
  (returns (CurrentStamina :type "Float (double-precision)"))
  (return (`/Game/DamageSystem/BPC_StatusComponent.CurrentStamina` (`self.BPC_StatusComponent`))))

(fn `GetMaxHealth`
  (returns (MaxHealth :type "Float (double-precision)"))
  (return (`/Game/DamageSystem/BPC_StatusComponent.MaxHealth` (`self.BPC_StatusComponent`))))

(fn `GetMaxStamina`
  (returns (MaxStamina :type "Float (double-precision)"))
  (return (`/Game/DamageSystem/BPC_StatusComponent.MaxStamina` (`self.BPC_StatusComponent`))))

(fn `Heal`
  (params (Amount :type "Float (double-precision)"))
  (returns (NewHealth :type "Float (double-precision)"))
  (bind _newhealth (`/Game/DamageSystem/BPC_StatusComponent.Heal` (`self.BPC_StatusComponent`) Amount))
  (return _newhealth))

(fn `TakeDamage`
  (params (DamageInfo :type "/Game/DamageSystem/S_Damage_Info Structure"))
  (returns (WasDamaged :type Boolean))
  (bind _wasdamaged (`/Game/DamageSystem/BPC_StatusComponent.TakeDamage` (`self.BPC_StatusComponent`) DamageInfo))
  (return _wasdamaged))

(fn `UserConstructionScript`
  (bind _bpc_statuscomponent (`self.BPC_StatusComponent`))
  (add `/Game/DamageSystem/BPC_StatusComponent.OnBlocked` _bpc_statuscomponent (`|CreateDelegate` :!event `DamageBlocked`))
  (add `/Game/DamageSystem/BPC_StatusComponent.OnDamageResponse` _bpc_statuscomponent (`|CreateDelegate` :!event `DamageReaction`))
  (add `/Game/DamageSystem/BPC_StatusComponent.OnDeath` _bpc_statuscomponent (`|CreateDelegate` :!event `Death`)))