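; GA_Block is a gameplay ability that puts a BP_BaseCharacter into a blocking state.
; On activation it commits, applies the GE_IsBlocking effect to the owner and calls Blocking on the character.
; It then waits for the Character.IsBlocking tag to be removed and ends itself.
; On end it calls FinishedBlocking and cleans up the tag-wait task.
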(event `self.K2_ActivateAbility`
  (`self.K2_CommitAbility`)
  (`self.BP_ApplyGameplayEffectToOwner` "/Game/Experience/Blueprints/Abilities/GE_IsBlocking.GE_IsBlocking_C")
  (bind _asbp_base_character (cast `/Game/ThirdPerson/Blueprints/BP_BaseCharacter` (`.OwnerActor` (break `GameplayAbilityActorInfo` (`self.GetActorInfo`)))))
  (`/Game/ThirdPerson/Blueprints/BP_BaseCharacter.Blocking` _asbp_base_character)
  (bind _asynctaskproxy (`AbilityTask_WaitGameplayTagRemoved.WaitGameplayTagRemove` (struct :`TagName` "Character.IsBlocking") null)
    (:`then`
      (set `self.Async Task` _asynctaskproxy))
    (:`Removed`
      (`self.K2_EndAbility`))))

(event `self.K2_OnEndAbility`
  (params (bWasCancelled :type Boolean))
  (bind _async_task (`self.Async Task`))
  (`/Game/ThirdPerson/Blueprints/BP_BaseCharacter.FinishedBlocking` (stale `self.K2_ActivateAbility` _asbp_base_character))
  (`/Engine/EditorBlueprintResources/StandardMacros.IsValid` _async_task
    (:`Is Valid`
      (`GameplayTask.EndTask` _async_task))))