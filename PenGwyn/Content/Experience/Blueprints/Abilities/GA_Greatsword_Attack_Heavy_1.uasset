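; Gameplay ability for the player's greatsword heavy attack, which spends stamina and plays one of three montages chosen by the character's combo count.
; It aligns the character to the camera when locked on and gates movement input around the montage length, with an attack sound on start.
; Montage completion, blend-out or interruption ends the ability, starts stamina regen, then calls the combo increase and reset in succession.
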(event `self.K2_ActivateAbility`
  (bind (_owneractor _avataractor _playercontroller _abilitysystemcomponent _skeletalmeshcomponent) (break `GameplayAbilityActorInfo` (`self.GetActorInfo`)))
  (`self.K2_CommitAbility`)
  (bind _asbp_third_person_character (cast `/Game/ThirdPerson/Blueprints/BP_ThirdPersonCharacter` _owneractor))
  (`/Game/ThirdPerson/Blueprints/BP_ThirdPersonCharacter.ConsumeStamina` _asbp_third_person_character 20.0)
  (bind _anim (`self.SelectAnimation` (`/Game/ThirdPerson/Blueprints/BP_ThirdPersonCharacter.ComboCount` _asbp_third_person_character))
    (:`Out`
      (if (`/Game/Experience/Blueprints/Components/BPC_TargetLockOnComponent.LockedOn` (`/Game/ThirdPerson/Blueprints/BP_ThirdPersonCharacter.BPC_TargetLockOnComponent` _asbp_third_person_character))
        (`/Game/ThirdPerson/Blueprints/BP_ThirdPersonCharacter.Align to Camera` _asbp_third_person_character))
      (`/Game/ThirdPerson/Blueprints/BP_ThirdPersonCharacter.MovmentInputHandler` _asbp_third_person_character 0.0 true)
      (`|PlayMontage` _skeletalmeshcomponent _anim
        (:`then`
          (`GameplayStatics.PlaySound2D` "/Game/Experience/Sound/SC_PlayerAttack.SC_PlayerAttack" 1.0 1.0 0.0 null null)
          (`/Game/ThirdPerson/Blueprints/BP_ThirdPersonCharacter.MovmentInputHandler` _asbp_third_person_character (`AnimationAsset.GetPlayLength` _anim) false))
        (:`OnCompleted`
          (`self.K2_EndAbility` :!label _label)
          (`/Game/ThirdPerson/Blueprints/BP_ThirdPersonCharacter.BeginStaminaRegen` _asbp_third_person_character)
          (`/Game/ThirdPerson/Blueprints/BP_ThirdPersonCharacter.Increase Combo Count` _asbp_third_person_character)
          (`/Game/ThirdPerson/Blueprints/BP_ThirdPersonCharacter.ResetComboCount` _asbp_third_person_character))
        (:`OnBlendOut`
          (goto _label))
        (:`OnInterrupted`
          (goto _label))))))