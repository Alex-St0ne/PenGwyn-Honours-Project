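; GA_Jump is a gameplay ability that makes the owning BP_ThirdPersonCharacter jump at a stamina cost.
; On activation it consumes a fixed amount of stamina, calls Jump, and plays the heavy jump sound if half the remaining stamina is above zero, otherwise the light one.
; It commits only after these effects, with no prior stamina check, then ends and starts stamina regeneration.
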(event `self.K2_ActivateAbility`
  (bind _asbp_third_person_character (cast `/Game/ThirdPerson/Blueprints/BP_ThirdPersonCharacter` (`.OwnerActor` (break `GameplayAbilityActorInfo` (`self.GetActorInfo`)))))
  (`/Game/ThirdPerson/Blueprints/BP_ThirdPersonCharacter.ConsumeStamina` _asbp_third_person_character 10.0)
  (`Character.Jump` _asbp_third_person_character)
  (if (< 0.0 (/ (`/Game/DamageSystem/BPC_StatusComponent.CurrentStamina` (`/Game/ThirdPerson/Blueprints/BP_ThirdPersonCharacter.BPC_StatusComponent` _asbp_third_person_character)) 2.0))
    (`GameplayStatics.PlaySound2D` "/Game/Experience/Sound/SC_PlayerJumpHeavy.SC_PlayerJumpHeavy" 1.0 1.0 0.0 null null)
    (else
      (`GameplayStatics.PlaySound2D` "/Game/Experience/Sound/SC_PlayerJumpLight.SC_PlayerJumpLight" 1.0 1.0 0.0 null null)))
  (`self.K2_CommitAbility`)
  (`self.K2_EndAbility`)
  (`/Game/ThirdPerson/Blueprints/BP_ThirdPersonCharacter.BeginStaminaRegen` _asbp_third_person_character))