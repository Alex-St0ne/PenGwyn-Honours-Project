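; Gameplay Ability that makes the third-person character perform a stamina-costed dodge roll.
; On activation it applies GE_IsRolling, consumes stamina, sets rolling and rotate-to-direction flags, and plays the character's roll montage.
; Montage completion, blend-out or interruption ends the ability, clears rolling flags, calls the input buffer and starts stamina regen; ending removes the rolling effect by tag.
; BP_PenGwynAssistant logs attempts, stamina use and non-interrupted rolls as successes.
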(event `self.K2_ActivateAbility`
  (bind (_owneractor _avataractor _playercontroller _abilitysystemcomponent _skeletalmeshcomponent) (break `GameplayAbilityActorInfo` (`self.GetActorInfo`)))
  ;[0 1 0.04705] Data Log
  (bind _returnvalue (`GameplayStatics.GetActorOfClass` "/Game/AssistiveControlScheme/BP_PenGwynAssistant.BP_PenGwynAssistant_C"))
  (message `/Game/AssistiveControlScheme/BPI_DataLogging.UpdateNumOfRollAttempts` _returnvalue)
  (`self.K2_CommitAbility`)
  (`self.BP_ApplyGameplayEffectToOwner` "/Game/Experience/Blueprints/Abilities/GE_IsRolling.GE_IsRolling_C")
  (bind _asbp_third_person_character (cast `/Game/ThirdPerson/Blueprints/BP_ThirdPersonCharacter` _owneractor))
  (`/Game/ThirdPerson/Blueprints/BP_ThirdPersonCharacter.ConsumeStamina` _asbp_third_person_character (`self.StaminaCost`))
  (set `/Game/ThirdPerson/Blueprints/BP_ThirdPersonCharacter.IsRolling` true _asbp_third_person_character)
  (set `/Game/ThirdPerson/Blueprints/BP_ThirdPersonCharacter.RoataToDirection` true _asbp_third_person_character)
  (`|PlayMontage` _skeletalmeshcomponent (`/Game/ThirdPerson/Blueprints/BP_ThirdPersonCharacter.RollAnimation` _asbp_third_person_character)
    (:`then`
      ;[0 1 0.04705] Data Log
      (bind _returnvalue_2 (`GameplayStatics.GetActorOfClass` "/Game/AssistiveControlScheme/BP_PenGwynAssistant.BP_PenGwynAssistant_C"))
      (message `/Game/AssistiveControlScheme/BPI_DataLogging.UpdateNumOfRollAttempts` _returnvalue_2)
      (message `/Game/AssistiveControlScheme/BPI_DataLogging.UpdateRollingStamina` _returnvalue_2 (`self.StaminaCost`)))
    (:`OnCompleted`
      (bind _returnvalue_3 (`GameplayStatics.GetActorOfClass` "/Game/AssistiveControlScheme/BP_PenGwynAssistant.BP_PenGwynAssistant_C" :!label _label))
      (message `/Game/AssistiveControlScheme/BPI_DataLogging.UpdateNumOfSuccessfullRolls` _returnvalue_3)
      (`self.K2_EndAbility` :!label _label_2)
      (set `/Game/ThirdPerson/Blueprints/BP_ThirdPersonCharacter.IsRolling` false _asbp_third_person_character)
      (set `/Game/Experience/ABP_AshenTwo.IsRolling` false (`/Game/ThirdPerson/Blueprints/BP_ThirdPersonCharacter.AnimBP` _asbp_third_person_character))
      (`/Game/ThirdPerson/Blueprints/BP_ThirdPersonCharacter.Input buffer` _asbp_third_person_character null true)
      (`/Game/ThirdPerson/Blueprints/BP_ThirdPersonCharacter.BeginStaminaRegen` _asbp_third_person_character))
    (:`OnBlendOut`
      (goto _label))
    (:`OnInterrupted`
      (goto _label_2))))

(event `self.K2_OnEndAbility`
  (params (bWasCancelled :type Boolean))
  (`self.BP_RemoveGameplayEffectFromOwnerWithGrantedTags` (struct :`GameplayTags` (struct :`(TagName` "Player.IsRolling")))))