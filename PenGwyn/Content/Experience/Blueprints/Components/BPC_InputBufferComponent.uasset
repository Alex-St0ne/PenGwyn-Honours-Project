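; Actor component that keeps a list of named input buffers, each linking an input to record with an action to perform.
; Functions add or remove entries, look them up by input action, and set or query an AlreadySet flag by buffer name.
; Executing a buffer broadcasts OnActionExecuted with its name and action, without checking or clearing the flag.
; The event graph is empty, so all logic runs only when called externally.
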(fn `CheckInputBufferInfoForActions`
  (params (BufferName :type Name))
  (returns (`Return Value` :type Boolean))
  (for _array_element (`self.InputBufferInfo`)
    (bind (_buffername _type _inputtorecord _actiontoperform _alreadyset) (break `/Game/Experience/Blueprints/Components/S_InputBufferInfo` _array_element))
    (if (and (== _buffername BufferName) _alreadyset)
      (return true)))
  (return false))

(fn `CreateNewInputBuffer`
  (params (`new input buffer info` :type "/Game/Experience/Blueprints/Components/S_InputBufferInfo Structure"))
  (`KismetArrayLibrary.Array_Add` (`self.InputBufferInfo`) `new input buffer info`))

(fn `ExecuteActionFromBuffer`
  (params (BufferName :type Name))
  (for _array_element (`self.InputBufferInfo`)
    (bind (_buffername _type _inputtorecord _actiontoperform) (break `/Game/Experience/Blueprints/Components/S_InputBufferInfo` _array_element))
    (if (== _buffername BufferName)
      (`self.OnActionExecuted` _buffername _actiontoperform)
      (return))))

(fn `RemoveInputBuffer`
  (params (name :type Name))
  (locals (LocalIndex :type Integer :default -1))
  (for (_array_element _array_index) (`self.InputBufferInfo`)
    (if (== (`.BufferName_2_0DAF3BAD4AD1AFB34ABCE29DF29BA4C7` (break `/Game/Experience/Blueprints/Components/S_InputBufferInfo` _array_element)) name)
      (set `local.LocalIndex` _array_index)))
  (if (!= (`local.LocalIndex`) -1)
    (`KismetArrayLibrary.Array_Remove` (`self.InputBufferInfo`) (`local.LocalIndex`))))

(fn `SearchForBufferOfInputAction`
  (params (InputAction :type "Object Object Reference"))
  (returns (ReturnValue :type Boolean) (`Array Index` :type Integer))
  (for (_array_element _array_index) (`self.InputBufferInfo`)
    (if (== (`.InputToRecord_10_55E75CCB4D89FBF04A3C7CAB0620EEBD` (break `/Game/Experience/Blueprints/Components/S_InputBufferInfo` _array_element)) InputAction)
      (return true _array_index)))
  (return false -1))

(fn `Set InputForBufferName`
  (params (BufferName :type Name))
  (locals (LocalIndex :type Integer :default -1))
  (bind _localindex (`local.LocalIndex`))
  (for (_array_element _array_index) (`self.InputBufferInfo`)
    (if (== (`.BufferName_2_0DAF3BAD4AD1AFB34ABCE29DF29BA4C7` (break `/Game/Experience/Blueprints/Components/S_InputBufferInfo` _array_element)) BufferName)
      (set `local.LocalIndex` _array_index)))
  (if (!= _localindex -1)
    (setmembers `/Game/Experience/Blueprints/Components/S_InputBufferInfo` :`StructRef` (`|GetArrayItem` (`self.InputBufferInfo`) _localindex) :`AlreadySet` true)))