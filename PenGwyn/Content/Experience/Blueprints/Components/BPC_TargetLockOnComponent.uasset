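; Souls-style target lock-on component for the player character that keeps the camera on a chosen enemy and marks it with an icon.
; Sphere trace gathers candidates, then line trace and camera-forward dot product pick the most centred.
; A looping timer eases control rotation toward the target with distance-based tilt, respawning the icon each tick, until out of radius.
; Left/right switching filters candidates by hit normal against camera right vector.
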(event `self.ReceiveBeginPlay`
  (set `self.PlayerRef` (cast `/Game/ThirdPerson/Blueprints/BP_ThirdPersonCharacter` (`GameplayStatics.GetPlayerCharacter` 0) :!pure true)))

(event `End Target Lock On`
  (set `self.LockedOn` false)
  (`KismetSystemLibrary.K2_ClearAndInvalidateTimerHandle` (stale `TriggerTargetLockOn` _returnvalue))
  (bind _lockonicon (`self.LockOnIcon`)
    (:`then`
      (`Actor.K2_DestroyActor` _lockonicon))
    (:`else`)))

(event `TriggerTargetLockOn`
  (bind _targettolockonto (`self.CheckForClosestTarget` (`self.TraceForTargets`)))
  (`/Engine/EditorBlueprintResources/StandardMacros.IsValid` _targettolockonto
    (:`Is Valid`
      (set `self.TargetLockedOn` _targettolockonto)
      (bind _returnvalue (`KismetSystemLibrary.K2_SetTimerDelegate` (delegate `Target Lock On`) (`GameplayStatics.GetWorldDeltaSeconds`) true)))))

(event `Target Lock On`
  (bind _returnvalue (`Pawn.GetController` (`self.PlayerRef`)))
  (bind _returnvalue_2 (`Controller.GetControlRotation` _returnvalue))
  (bind (_returnvalue_roll _returnvalue_pitch _returnvalue_yaw) (`KismetMathLibrary.BreakRotator` (`KismetMathLibrary.RInterpTo` _returnvalue_2 (`self.GetLockOnCameraRotation`) 0.01 10.0)))
  (if (> (`KismetMathLibrary.Vector_Distance` (`Actor.K2_GetActorLocation` (`self.PlayerRef`)) (`Actor.K2_GetActorLocation` (`self.TargetLockedOn`))) (`self.LockOnRadius`))
    (`self.End Target Lock On`)
    (else
      (set `self.LockedOn` true)
      (`Controller.SetControlRotation` _returnvalue (`KismetMathLibrary.MakeRotator` (.roll _returnvalue_2) _returnvalue_pitch _returnvalue_yaw))
      (`self.AddLockOnIcon`))))

(event `Switch Target On Left`
  (`/Engine/EditorBlueprintResources/StandardMacros.IsValid` (`self.TargetLockedOn`)
    (:`Is Valid`
      (bind _lefttarget (`self.GetTargetOnLeft`))
      (`/Engine/EditorBlueprintResources/StandardMacros.IsValid` _lefttarget
        (:`Is Valid`
          (set `self.TargetLockedOn` _lefttarget)
          (`self.AddLockOnIcon` :!label _label))))))

(event `Switch Target On Right`
  (`/Engine/EditorBlueprintResources/StandardMacros.IsValid` (`self.TargetLockedOn`)
    (:`Is Valid`
      (bind _lefttarget (`self.GetTargetOnRight`))
      (`/Engine/EditorBlueprintResources/StandardMacros.IsValid` _lefttarget
        (:`Is Valid`
          (set `self.TargetLockedOn` _lefttarget)
          (goto _label))))))

(event `AddLockOnIcon`
  (bind _targetlockedon (`self.TargetLockedOn`)
    (:`then`
      (bind _lockonicon (`self.LockOnIcon`)
        (:`then`
          (`Actor.K2_DestroyActor` _lockonicon))
        (:`else`
          _))
      (bind _returnvalue (`|SpawnActorFromClass` "/Game/UI/Widgits/BP_LockOnIcon.BP_LockOnIcon_C" (`SceneComponent.K2_GetComponentToWorld` (`/Game/Experience/Blueprints/AI/BP_Enemy_Base.LockOnPoint` (cast `/Game/Experience/Blueprints/AI/BP_Enemy_Base` _targetlockedon :!pure true))) "Undefined" "MultiplyWithRoot" null null))
      (set `self.LockOnIcon` _returnvalue))
    (:`else`
      (bind _lockonicon_2 (`self.LockOnIcon`)
        (:`then`
          (`Actor.K2_DestroyActor` _lockonicon_2))
        (:`else`)))))

(fn `CheckForClosestTarget`
  (params (Targets :type "Array of Actor Object Reference"))
  (returns (TargetToLockOnTo :type "Actor Object Reference"))
  (locals (LocalCompareFloat :type "Float (double-precision)") (LocalTargetToLcokOnTo :type "Actor Object Reference"))
  (for _array_element Targets
    (bind (_outhit _returnvalue) (`KismetSystemLibrary.LineTraceSingle` (`SceneComponent.K2_GetComponentLocation` (`PenGwynCharacter.FollowCamera` (`self.PlayerRef`))) (`Actor.K2_GetActorLocation` _array_element) "TraceTypeQuery1"))
    (if _returnvalue
      (bind _returnvalue_2 (`self.CheckRangeFromCenter` _array_element))
      (`/Engine/EditorBlueprintResources/StandardMacros.CompareFloat` _returnvalue_2 (`local.LocalCompareFloat`)
        (:`>`
          (set `local.LocalCompareFloat` _returnvalue_2)
          (set `local.LocalTargetToLcokOnTo` _array_element)))))
  (return (`local.LocalTargetToLcokOnTo`)))

(fn `CheckRangeFromCenter`
  (params (Target :type "Actor Object Reference"))
  (returns (ReturnValue :type "Float (double-precision)"))
  (bind _playerref (`self.PlayerRef`))
  (return (`KismetMathLibrary.Dot_VectorVector` (`SceneComponent.GetForwardVector` (`PenGwynCharacter.FollowCamera` _playerref)) (`KismetMathLibrary.Conv_RotatorToVector` (`KismetMathLibrary.FindLookAtRotation` (`Actor.K2_GetActorLocation` _playerref) (`Actor.K2_GetActorLocation` Target))))))

(fn `GetLockOnCameraRotation`
  (returns (Rotation :type "Rotator Structure"))
  (bind (_returnvalue_x _returnvalue_y _returnvalue_z) (`KismetMathLibrary.BreakVector` (`Actor.K2_GetActorLocation` (`self.TargetLockedOn`))))
  (return (`KismetMathLibrary.FindLookAtRotation` (`SceneComponent.K2_GetComponentLocation` (`PenGwynCharacter.FollowCamera` (`self.PlayerRef`))) (`KismetMathLibrary.MakeVector` _returnvalue_x _returnvalue_y (- _returnvalue_z (/ (`KismetMathLibrary.Vector_Distance` (`Actor.K2_GetActorLocation` (`self.PlayerRef`)) (`Actor.K2_GetActorLocation` (`self.TargetLockedOn`))) (`self.CameraTilt`)))))))

(fn `GetTargetLockedOnTo`
  (returns (TargetLockedOn :type "Actor Object Reference"))
  (return (`self.TargetLockedOn`)))

(fn `GetTargetOnLeft`
  (returns (LeftTarget :type "Actor Object Reference"))
  (locals (LocalTargetCompareFloat :type "Float (double-precision)") (LocalTargetToLockOnTarget :type "Actor Object Reference"))
  (for _array_element (`self.TraceForTargets`)
    (bind (_outhit _returnvalue) (`KismetSystemLibrary.LineTraceSingleForObjects` (`SceneComponent.K2_GetComponentLocation` (`PenGwynCharacter.FollowCamera` (`self.PlayerRef`))) (`Actor.K2_GetActorLocation` _array_element) (`|MakeArray` "ObjectTypeQuery7" :!type "EObjectTypeQuery Enum")))
    (if _returnvalue
      (if (and (!= (`self.TargetLockedOn`) _array_element) (> (`KismetMathLibrary.DegAsin` (`KismetMathLibrary.Dot_VectorVector` (`SceneComponent.GetRightVector` (`PenGwynCharacter.FollowCamera` (`self.PlayerRef`))) (`.Normal` (`GameplayStatics.BreakHitResult` _outhit)))) 0.0))
        (bind _returnvalue_2 (`self.CheckRangeFromCenter` _array_element))
        (`/Engine/EditorBlueprintResources/StandardMacros.CompareFloat` _returnvalue_2 (`local.LocalTargetCompareFloat`)
          (:`>`
            (set `local.LocalTargetCompareFloat` _returnvalue_2)
            (set `local.LocalTargetToLockOnTarget` _array_element))))))
  (return (`local.LocalTargetToLockOnTarget`)))

(fn `GetTargetOnRight`
  (returns (LeftTarget :type "Actor Object Reference"))
  (locals (LocalTargetCompareFloat :type "Float (double-precision)") (LocalTargetToLockOnTarget :type "Actor Object Reference"))
  (for _array_element (`self.TraceForTargets`)
    (bind (_outhit _returnvalue) (`KismetSystemLibrary.LineTraceSingleForObjects` (`SceneComponent.K2_GetComponentLocation` (`PenGwynCharacter.FollowCamera` (`self.PlayerRef`))) (`Actor.K2_GetActorLocation` _array_element) (`|MakeArray` "ObjectTypeQuery7" :!type "EObjectTypeQuery Enum")))
    (if _returnvalue
      (if (and (!= (`self.TargetLockedOn`) _array_element) (< (`KismetMathLibrary.DegAsin` (`KismetMathLibrary.Dot_VectorVector` (`SceneComponent.GetRightVector` (`PenGwynCharacter.FollowCamera` (`self.PlayerRef`))) (`.Normal` (`GameplayStatics.BreakHitResult` _outhit)))) 0.0))
        (bind _returnvalue_2 (`self.CheckRangeFromCenter` _array_element))
        (`/Engine/EditorBlueprintResources/StandardMacros.CompareFloat` _returnvalue_2 (`local.LocalTargetCompareFloat`)
          (:`>`
            (set `local.LocalTargetCompareFloat` _returnvalue_2)
            (set `local.LocalTargetToLockOnTarget` _array_element))))))
  (return (`local.LocalTargetToLockOnTarget`)))

(fn `TraceForTargets`
  (returns (Targets :type "Array of Actor Object Reference"))
  (locals (LocalTargets :type "Array of Actor Object Reference"))
  (bind _returnvalue (`Actor.K2_GetActorLocation` (`self.PlayerRef`)))
  (bind (_outhits _returnvalue_2) (`KismetSystemLibrary.SphereTraceMultiForObjects` _returnvalue _returnvalue (`self.LockOnRadius`) (`|MakeArray` "ObjectTypeQuery7" :!type "EObjectTypeQuery Enum")))
  (if _returnvalue_2
    (for _array_element _outhits
      (bind (_bblockinghit _binitialoverlap _time _distance _location _impactpoint _normal _impactnormal _physmat _hitactor) (`GameplayStatics.BreakHitResult` _array_element))
      (if (`KismetMathLibrary.ClassIsChildOf` (`GameplayStatics.GetObjectClass` _hitactor) (`self.LockOnClass`))
        (`KismetArrayLibrary.Array_Add` (`local.LocalTargets`) _hitactor)))
    (return (`local.LocalTargets`))))