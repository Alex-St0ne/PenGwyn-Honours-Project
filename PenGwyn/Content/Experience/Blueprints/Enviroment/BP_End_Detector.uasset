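; BP_End_Detector is a level actor that ends the game once its tracked enemies are gone.
; On BeginPlay it gathers three enemy references into an Enemies array.
; Its EndLevel event scans that array with IsValid, stops at the first surviving enemy, and opens the EndGame level when none remain.
; EndLevel is not triggered within this graph, as overlap and tick are unused.
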(event `self.ReceiveBeginPlay`
  (`KismetArrayLibrary.Array_Add` (`self.Enemies`) (`self.Enemy_0`))
  (`KismetArrayLibrary.Array_Add` (`self.Enemies`) (`self.Enemy_1`))
  (`KismetArrayLibrary.Array_Add` (`self.Enemies`) (`self.Enemy_2`)))

(event `EndLevel`
  (for _array_element (`self.Enemies`)
    (bind _output_get (set `self.EnemyAlive` (`KismetSystemLibrary.IsValid` _array_element)))
    (if _output_get
      (break)))
  (if (not (`self.EnemyAlive`))
    (`GameplayStatics.OpenLevel` "EndGame")))

(fn `UserConstructionScript`)