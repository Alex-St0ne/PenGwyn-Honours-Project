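; BP_FogWall is a fog wall that can be removed once its three assigned enemies are gone.
; On player overlap it shows an interact prompt, though that check tests only the first enemy's validity.
; Activate checks all three, then plays a sound, calls UpdateAssistance on BP_PenGwynAssistant and destroys the wall after a short delay.
; A flag prevents repeat activation.
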(event `self.ReceiveBeginPlay`
  (`KismetArrayLibrary.Array_Add` (`self.Enemies`) (`self.Enemy1`))
  (`KismetArrayLibrary.Array_Add` (`self.Enemies`) (`self.Enemy2`))
  (`KismetArrayLibrary.Array_Add` (`self.Enemies`) (`self.Enemy3`)))

(event `self.Box.OnComponentBeginOverlap`
  (params (OverlappedComponent :type "PrimitiveComponent Object Reference") (OtherActor :type "Actor Object Reference") (OtherComp :type "PrimitiveComponent Object Reference") (OtherBodyIndex :type Integer) (bFromSweep :type Boolean) (SweepResult :type "HitResult Structure (by ref)"))
  (if (== OtherActor (`GameplayStatics.GetPlayerCharacter` 0))
    (for _array_element (`self.Enemies`)
      (set `self.EnemyAlive` (`KismetSystemLibrary.IsValid` _array_element))
      (break))
    (if (not (`self.EnemyAlive`))
      (`SceneComponent.SetVisibility` (`self.InteractPrompt`) true false))))

(event `self.Box.OnComponentEndOverlap`
  (params (OverlappedComponent :type "PrimitiveComponent Object Reference") (OtherActor :type "Actor Object Reference") (OtherComp :type "PrimitiveComponent Object Reference") (OtherBodyIndex :type Integer))
  (`SceneComponent.SetVisibility` (`self.InteractPrompt`) false false))

(event `Activate`
  (if (not (`self.Began Assesment`))
    (for _array_element (`self.Enemies`)
      (bind _output_get (set `self.EnemyAlive` (`KismetSystemLibrary.IsValid` _array_element)))
      (if _output_get
        (break)))
    (if (not (`self.EnemyAlive`))
      (`GameplayStatics.PlaySound2D` "/Game/Experience/Sound/SC_FogWallActivated.SC_FogWallActivated" 1.0 1.0 0.0 null null)
      (set `self.Began Assesment` true)
      (bind _returnvalue (`GameplayStatics.GetActorOfClass` "/Game/AssistiveControlScheme/BP_PenGwynAssistant.BP_PenGwynAssistant_C"))
      (`/Game/AssistiveControlScheme/BP_PenGwynAssistant.UpdateAssistance` _returnvalue)
      (`KismetSystemLibrary.Delay` 1.0)
      (`self.K2_DestroyActor`))))

(event `self.ReceiveDestroyed`)

(fn `UserConstructionScript`)