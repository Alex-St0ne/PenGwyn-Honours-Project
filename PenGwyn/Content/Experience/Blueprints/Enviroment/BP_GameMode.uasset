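; Game mode that spawns and possesses the third-person player character, then resets the enemies of that character's room.
; The stored room ID selects a hardcoded set of light and heavy enemies, each with its behavior tree.
; For each enemy ID, a helper resets the existing enemy and spawns a replacement AI at the matching spawner.
; Replacement only happens when an enemy with that ID is found in the world.
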(event `/Game/Experience/Blueprints/Enviroment/BPI_GameManager.SpawnPlayer`
  (params (Transform :type "Transform Structure") (RoomID :type Integer))
  (set `self.RoomId` RoomID)
  (bind _returnvalue (`|SpawnActorFromClass` "/Game/ThirdPerson/Blueprints/BP_ThirdPersonCharacter.BP_ThirdPersonCharacter_C" Transform "Undefined" "MultiplyWithRoot" null null))
  (`Controller.Possess` (`GameplayStatics.GetPlayerController` 0) _returnvalue)
  (`self.ResetEnemies`))

(event `/Game/Experience/Blueprints/Enviroment/BPI_GameManager.Reset Enemy`
  (`self.ResetEnemies`))

(event `ResetEnemies`
  (switch `int` (`self.RoomId`)
    (:`0`
      (`self.DestroyAndResetEnmey` 0 "/Game/Experience/Blueprints/AI/BP_Enemy_Light.BP_Enemy_Light_C" "/Game/Experience/Blueprints/AI/Behaviour/BT_Enemy_Light.BT_Enemy_Light"))
    (:`1`
      (`self.DestroyAndResetEnmey` 1 "/Game/Experience/Blueprints/AI/BP_Enemy_Heavy.BP_Enemy_Heavy_C" "/Game/Experience/Blueprints/AI/Behaviour/BT_Enemy_Heavy.BT_Enemy_Heavy"))
    (:`2`
      (`self.DestroyAndResetEnmey` 2 "/Game/Experience/Blueprints/AI/BP_Enemy_Light.BP_Enemy_Light_C" "/Game/Experience/Blueprints/AI/Behaviour/BT_Enemy_Light.BT_Enemy_Light")
      (`self.DestroyAndResetEnmey` 3 "/Game/Experience/Blueprints/AI/BP_Enemy_Light.BP_Enemy_Light_C" "/Game/Experience/Blueprints/AI/Behaviour/BT_Enemy_Light.BT_Enemy_Light"))
    (:`3`
      (`self.DestroyAndResetEnmey` 4 "/Game/Experience/Blueprints/AI/BP_Enemy_Light.BP_Enemy_Light_C" "/Game/Experience/Blueprints/AI/Behaviour/BT_Enemy_Light.BT_Enemy_Light")
      (`self.DestroyAndResetEnmey` 5 "/Game/Experience/Blueprints/AI/BP_Enemy_Light.BP_Enemy_Light_C" "/Game/Experience/Blueprints/AI/Behaviour/BT_Enemy_Light.BT_Enemy_Light")
      (`self.DestroyAndResetEnmey` 6 "/Game/Experience/Blueprints/AI/BP_Enemy_Heavy.BP_Enemy_Heavy_C" "/Game/Experience/Blueprints/AI/Behaviour/BT_Enemy_Heavy.BT_Enemy_Heavy"))))

(fn `UserConstructionScript`)